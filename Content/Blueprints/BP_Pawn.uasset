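; BP_Pawn is a flyable P-38 aircraft pawn that constantly moves along its forward vector and fires rockets.
; BeginPlay registers both propeller meshes with a rotate component to spin them.
; A combined Enhanced Input pitch-and-roll action applies delta-time-scaled local rotation, leaving the separate pitch and roll actions unused.
; Firing spawns BP_Rocket at the left launch point, then at the right after a short delay.
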(event Input|EnhancedActionEvents|EnhancedInputActionIA_Pitch
  (params (ActionValue :type Float%20%28double-precision%29) (ElapsedSeconds :type Float%20%28double-precision%29) (TriggeredSeconds :type Float%20%28double-precision%29) (InputAction :type Input%20Action%20Object%20Reference :default "/Game/Blueprints/Inputs/IA_Pitch.IA_Pitch"))
  ;[1 1 1] NotUse
)

(event Input|EnhancedActionEvents|EnhancedInputActionIA_Roll
  (params (ActionValue :type Float%20%28double-precision%29) (ElapsedSeconds :type Float%20%28double-precision%29) (TriggeredSeconds :type Float%20%28double-precision%29) (InputAction :type Input%20Action%20Object%20Reference :default "/Game/Blueprints/Inputs/IA_Roll.IA_Roll"))
  ;[1 1 1] NotUse
)

(event Input|EnhancedActionEvents|EnhancedInputActionIA_PitchnRoll
  (params (ActionValue :type Vector%202D%20Structure) (ElapsedSeconds :type Float%20%28double-precision%29) (TriggeredSeconds :type Float%20%28double-precision%29) (InputAction :type Input%20Action%20Object%20Reference :default "/Game/Blueprints/Inputs/IA_PitchnRoll.IA_PitchnRoll"))
  (bind _returnvalue (Utilities|Time|GetWorldDeltaSeconds))
  (Transformation|AddActorLocalRotation (Math|Rotator|MakeRotator (* (.x ActionValue) _returnvalue 1e+02) (* (.y ActionValue) _returnvalue 1e+02) 0.0) false false))

(event Input|EnhancedActionEvents|EnhancedInputActionIA_Fire
  (params (ActionValue :type Boolean) (ElapsedSeconds :type Float%20%28double-precision%29) (TriggeredSeconds :type Float%20%28double-precision%29) (InputAction :type Input%20Action%20Object%20Reference :default "/Game/Blueprints/Inputs/IA_Fire.IA_Fire"))
  (Utilities|FlowControl|Sequence
    (:then_0
      (Game|SpawnActorfromClass "/Game/Blueprints/BP_Rocket.BP_Rocket_C" (Transformation|GetSocketTransform (Variables|Default|GetRocketFireLeft) "None" "RTS_World") "Undefined" "MultiplyWithRoot" 0 0))
    (:then_1
      (Utilities|FlowControl|Delay 0.5)
      (Game|SpawnActorfromClass "/Game/Blueprints/BP_Rocket.BP_Rocket_C" (Transformation|GetSocketTransform (Variables|Default|GetRocketFireRight) "None" "RTS_World") "Undefined" "MultiplyWithRoot" 0 0))))

(event EventBeginPlay
  (bind _ac_rotatecomponent (Variables|Default|GetAC_RotateComponent))
  (Utilities|FlowControl|Sequence
    (:then_0
      (Default|AddRotateFunction _ac_rotatecomponent (Variables|Default|GetSM_P38_PropellerLeft)))
    (:then_1
      (Default|AddRotateFunction _ac_rotatecomponent (Variables|Default|GetSM_P38_PropellerRight)))))

(event EventTick
  (params (DeltaSeconds :type Float%20%28single-precision%29))
  (Pawn|Input|AddMovementInput (Transformation|GetActorForwardVector) 1.0 false))

(fn ConstructionScript)